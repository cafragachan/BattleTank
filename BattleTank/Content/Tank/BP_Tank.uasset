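; Player-controllable tank pawn Blueprint that wires input to its movement and aiming components and links its health bar widget back to itself.
; BeginPlay passes both tracks to TankMovement1; the TankAiming initialisation with turret and barrel is left disconnected.
; Axis inputs drive movement intents and rotate the azimuth gimbal and spring arm, scaled by frame time.
; Fire goes to TankAiming, and SwapCamera toggles the first-person and other camera.
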(event EventBeginPlay
  (Class|TankMovementComponent|InitialiseMovement (Variables|Default|GetTankMovement1) (Variables|Default|GetRightTrack) (Variables|Default|GetLeftTrack))
  (bind _ashealth_bar (Utilities|Casting|CastToHealthBar (UserInterface|GetUserWidgetObject (Variables|Default|GetHealth%20Bar))))
  (Variables|/Game/UI/HealthBar.HealthBar_C|SetmyTank _ashealth_bar self))

(event Input|ActionEvents|InputActionFire
  (params (Key :type Key%20Structure))
  ;[1 1 1] Aim Movement
  (:Pressed
    (Class|TankAimingComponent|Fire (Variables|Default|GetTankAiming))))

(event Input|ActionEvents|InputActionSwapCamera
  (params (Key :type Key%20Structure))
  (:Pressed
    (Components|Activation|ToggleActive (Variables|Default|GetFirstPersonCamera))))

(event Input|AxisEvents|InputAxisAimAzimuth
  (params (AxisValue :type Float%20%28single-precision%29))
  ;[1 1 1] Aim Movement
  (Transformation|AddLocalRotation (Variables|Default|GetAzimuthGimbal) (Math|Rotator|MakeRotator 0.0 0.0 (* AxisValue (Utilities|Time|GetWorldDeltaSeconds) 1e+02)) false false))

(event Input|AxisEvents|InputAxisRight
  (params (AxisValue :type Float%20%28single-precision%29))
  ;[1 1 1] Tank Movement
  (Class|TankMovementComponent|IntendMoveRight (Variables|Default|GetTankMovement1) AxisValue))

(event Input|AxisEvents|InputAxisLeft
  (params (AxisValue :type Float%20%28single-precision%29))
  ;[1 1 1] Tank Movement
  (Class|TankMovementComponent|IntendMoveLeft (Variables|Default|GetTankMovement1) AxisValue))

(event Input|AxisEvents|InputAxisAimElevation
  (params (AxisValue :type Float%20%28single-precision%29))
  ;[1 1 1] Aim Movement
  (Transformation|AddLocalRotation (Variables|Default|GetSpringArm) (Math|Rotator|MakeRotator 0.0 (* AxisValue (Utilities|Time|GetWorldDeltaSeconds) 1e+02) 0.0) false false))

(event Input|AxisEvents|InputAxisForward
  (params (AxisValue :type Float%20%28single-precision%29))
  ;[1 1 1] Tank Movement
  (Class|TankMovementComponent|IntendMoveForward (Variables|Default|GetTankMovement1) AxisValue))

(fn ConstructionScript)

(fn BPInitialiseHealthWidget
  (bind _ashealth_bar (Utilities|Casting|CastToHealthBar (UserInterface|GetUserWidgetObject (Variables|Default|GetHealth%20Bar))))
  (Variables|/Game/UI/HealthBar.HealthBar_C|SetmyTank _ashealth_bar self))